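; Terrain tile for infinite terrain that scatters random props (containers, boxes, canisters, sandbags, rocks) via PlaceActors on BeginPlay and starts with its barrier locked.
; The player entering LockingVolume opens the barrier and turns it green; leaving relocks it in red and asks InfiniteTerrainGameMode to spawn tiles.
; The player touching DestroyVolume destroys the tile.
; GetAttachLocation exposes the Arrow's world transform as an attach point.
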(event OnComponentBeginOverlap(LockingVolume)
  (params (OverlappedComponent :type Primitive%20Component%20Object%20Reference) (OtherActor :type Actor%20Object%20Reference) (OtherComp :type Primitive%20Component%20Object%20Reference) (OtherBodyIndex :type Integer) (bFromSweep :type Boolean) (SweepResult :type Hit%20Result%20Structure%20%28by%20ref%29))
  (Utilities|IsPlayerActor OtherActor)
  (CallFunction|Unlock))

(event OnComponentEndOverlap(LockingVolume)
  (params (OverlappedComponent :type Primitive%20Component%20Object%20Reference) (OtherActor :type Actor%20Object%20Reference) (OtherComp :type Primitive%20Component%20Object%20Reference) (OtherBodyIndex :type Integer))
  (Utilities|IsPlayerActor OtherActor)
  (CallFunction|Lock)
  (bind _asinfinite_terrain_game_mode (Utilities|Casting|CastToInfiniteTerrainGameMode (Game|GetGameMode)))
  (Default|SpawnTiles _asinfinite_terrain_game_mode))

(event OnComponentBeginOverlap(DestroyVolume)
  (params (OverlappedComponent :type Primitive%20Component%20Object%20Reference) (OtherActor :type Actor%20Object%20Reference) (OtherComp :type Primitive%20Component%20Object%20Reference) (OtherBodyIndex :type Integer) (bFromSweep :type Boolean) (SweepResult :type Hit%20Result%20Structure%20%28by%20ref%29))
  (Utilities|IsPlayerActor OtherActor)
  (Actor|DestroyActor))

(event EventBeginPlay
  (CallFunction|Lock)
  (Class|Tile|PlaceActors "/Game/Dynamic/Terrain/Props/BP_Container.BP_Container_C" 1 3 5e+02 1.0 1.0)
  (Class|Tile|PlaceActors "/Game/Dynamic/Terrain/Props/BP_Box.BP_Box_C" 2 4 1e+02 1.0 1.0)
  (Class|Tile|PlaceActors "/Game/Dynamic/Terrain/Props/BP_Canister.BP_Canister_C" 1 3 5e+01 1.0 1.0)
  (Class|Tile|PlaceActors "/Game/Dynamic/Terrain/Props/BP_SandBags.BP_SandBags_C" 1 2 2.5e+02 1.0 1.0)
  (Class|Tile|PlaceActors "/Game/Dynamic/Terrain/Props/BP_Rock1.BP_Rock1_C" 1 5 1.5e+02 1.0 5.0)
  (Class|Tile|PlaceActors "/Game/Dynamic/Terrain/Props/BP_Rock2.BP_Rock2_C" 1 5 2.5e+02 1.0 5.0)
  (Class|Tile|PlaceActors "/Game/Dynamic/Terrain/Props/BP_Rock3.BP_Rock3_C" 1 5 2.5e+02 1.0 5.0))

(event Collision|EventActorBeginOverlap
  (params (OtherActor :type Actor%20Object%20Reference)))

(event EventTick
  (params (DeltaSeconds :type Float%20%28single-precision%29)))

(fn ConstructionScript)

(fn GetAttachLocation
  (return (Transformation|GetWorldTransform (Variables|Default|GetArrow))))

(fn Unlock
  (Collision|SetCollisionEnabled (Variables|Default|GetBarrier) "NoCollision")
  (Rendering|Material|SetMaterial (Variables|Default|GetBarrier) 0 "/Game/Dynamic/Terrain/MI_Barrier_Green.MI_Barrier_Green"))

(fn Lock
  (Collision|SetCollisionEnabled (Variables|Default|GetBarrier) "QueryAndPhysics")
  (Rendering|Material|SetMaterial (Variables|Default|GetBarrier) 0 "/Game/Dynamic/Terrain/MI_Barrier_Red.MI_Barrier_Red"))